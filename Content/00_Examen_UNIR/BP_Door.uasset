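; BP_Door is a double sliding door that opens only while every button in its Buttons array is pressed.
; On BeginPlay it stores both leaf positions, binds to each button's pressed-changed event and runs an initial check.
; Each change re-evaluates all buttons, then plays or reverses one Timeline.
; The Timeline lerps the leaves apart along local X, with a keyed curve meant to suggest a straining door.
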(event `self.ReceiveBeginPlay`
  ; Configuración inicial
  (set `self.LeftDoorPosIni` (`SceneComponent.RelativeLocation` (`self.LeftDoor`)))
  (set `self.RightDoorPosIni` (`SceneComponent.RelativeLocation` (`self.RightDoor`)))
  (for _array_element (`self.Buttons`)
    (add `/Game/00_Examen_UNIR/BP_FloorButton.OnPressedChanged` _array_element (delegate `ComprobarAbrirPuerta`)))
  (set `self.SePuedeAbrir` true :!label _label)
  (for _array_element_2 (`self.Buttons`)
    (if (not (`/Game/00_Examen_UNIR/BP_FloorButton.Pressed` _array_element_2))
      (set `self.SePuedeAbrir` false)))
  (if (`self.SePuedeAbrir`)
    (`self.OpenDoor`)
    (else
      (`self.CloseDoor`))))

(event `ComprobarAbrirPuerta`
  ; Configuración inicial
  (goto _label))

(event `OpenDoor`
  ; Eventos abrir y cerrar puerta
  (bind (_direction _newtrack_0) (`Timeline|Timeline` :!label _label_2) ; Se incluyen 3 keys para hacer el efecto como de que le cuesta abrirse
    (:`Update`
      (`SceneComponent.K2_SetRelativeLocation` (`self.LeftDoor`) (`KismetMathLibrary.VLerp` (`self.LeftDoorPosIni`) (+ (`self.LeftDoorPosIni`) (-80.0 0.0 0.0)) _newtrack_0) false false)
      (`SceneComponent.K2_SetRelativeLocation` (`self.RightDoor`) (`KismetMathLibrary.VLerp` (`self.RightDoorPosIni`) (+ (`self.RightDoorPosIni`) (80.0 0.0 0.0)) _newtrack_0) false false))))

(event `CloseDoor`
  ; Eventos abrir y cerrar puerta
  (goto _label_2 :!via `Reverse`))

(fn `UserConstructionScript`)