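; BP_FloorButton is a floor button that the player toggles with E while standing on it.
; Box overlaps with BP_ThirdPersonCharacter set PlayerInside and enable or disable the actor's input, and the key handler rechecks that flag.
; Each press flips Pressed, swaps the hieroglyph mesh's material and fires OnPressedChanged to signal the change.
; BeginPlay applies the material matching the initial Pressed value.
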(event `self.ReceiveBeginPlay`
  (bind _sm_hieroglyph_007 (`self.SM_hieroglyph_007`))
  ; Configuración inicial de los botones
  (if (`self.Pressed`)
    (`PrimitiveComponent.SetMaterial` _sm_hieroglyph_007 0 "/Game/00_Examen_UNIR/M_BotonApretado.M_BotonApretado")
    (else
      (`PrimitiveComponent.SetMaterial` _sm_hieroglyph_007 0 "/Game/00_Examen_UNIR/M_BotonNoApretado.M_BotonNoApretado"))))

(event `self.Box.OnComponentBeginOverlap`
  (params (OverlappedComponent :type "PrimitiveComponent Object Reference") (OtherActor :type "Actor Object Reference") (OtherComp :type "PrimitiveComponent Object Reference") (OtherBodyIndex :type Integer) (bFromSweep :type Boolean) (SweepResult :type "HitResult Structure (by ref)"))
  ; Detectar al jugador encima del botón
  (cast `/Game/ThirdPerson/Blueprints/BP_ThirdPersonCharacter` OtherActor)
  (set `self.PlayerInside` true)
  (`self.EnableInput` (`GameplayStatics.GetPlayerController` 0)))

(event `self.Box.OnComponentEndOverlap`
  (params (OverlappedComponent :type "PrimitiveComponent Object Reference") (OtherActor :type "Actor Object Reference") (OtherComp :type "PrimitiveComponent Object Reference") (OtherBodyIndex :type Integer))
  ; Detectar al jugador quitándose de encima del botón
  (cast `/Game/ThirdPerson/Blueprints/BP_ThirdPersonCharacter` OtherActor)
  (set `self.PlayerInside` false)
  (`self.DisableInput` (`GameplayStatics.GetPlayerController` 0)))

(event `Key|E`
  (params (Key :type "Key Structure"))
  (bind _sm_hieroglyph_007 (`self.SM_hieroglyph_007`))
  ; Gestión de presionar el botón
  (:`Pressed`
    (if (`self.PlayerInside`)
      (bind _output_get (set `self.Pressed` (not (`self.Pressed`))))
      (if _output_get
        (`PrimitiveComponent.SetMaterial` _sm_hieroglyph_007 0 "/Game/00_Examen_UNIR/M_BotonApretado.M_BotonApretado")
        (else
          (`PrimitiveComponent.SetMaterial` _sm_hieroglyph_007 0 "/Game/00_Examen_UNIR/M_BotonNoApretado.M_BotonNoApretado")))
      (`self.OnPressedChanged`))))

(fn `UserConstructionScript`)